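; Ship_Bp is the ship Blueprint, with a capsule, camera pivot and weapon spawn points, that ends the game when destroyed.
; On BeginPlay it registers its pivot and camera and passes tiered spawn points to the weapon setup, leaving some slots empty.
; Each Tick it compares current life against one and opens the Lose level when it drops below.
; The construction script assigns the ship model and capsule to its Ship and MyMesh variables.
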(event `self.ReceiveBeginPlay`
  (`self.SetCamera` (`self.Pivot`) (`self.Camera`))
  (`self.SetWeapons` (`|MakeArray` (`self.Spawn_1_T2`) null (`self.Spawn_1_T1`) (`self.Spawn_2_T1`) null (`self.Spawn_2_T3`) (`self.Spawn_3_T3`) (`self.Spawn_4_T3`) (`self.Spawn_5_T3`) null)))

(event `self.ReceiveTick`
  (params (DeltaSeconds :type "Float (single-precision)"))
  (`/Engine/EditorBlueprintResources/StandardMacros.CompareInt` (`self.currentLife`) 1
    (:`<`
      (`GameplayStatics.OpenLevel` "Lose"))))

(fn `UserConstructionScript`
  (set `self.ship` (`self.ShipModel`))
  (set `self.myMesh` (`self.CapsuleComponent`)))