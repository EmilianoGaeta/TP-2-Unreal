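; Wheel bomb Blueprint that shatters into a destructible mesh once its IDied flag is set.
; The construction script assigns WheelBall to the Weel and Bomb references and Capsule to Mesh.
; Tick polls IDied and, while true, swaps WheelBall for WheelBallDM, applies fracturing radius damage and disables Sphere and Capsule collision.
; This repeats every frame because nothing here gates it to run once.
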(event `self.ReceiveTick`
  (params (DeltaSeconds :type "Float (single-precision)"))
  (bind _idied (`self.iDied`))
  (if _idied
    (`SceneComponent.SetVisibility` (`self.WheelBall`) (not _idied) false)
    (`SceneComponent.SetVisibility` (`self.WheelBall_DM`) _idied false)
    (`DestructibleComponent.ApplyRadiusDamage` (`self.WheelBall_DM`) 0.0 (`self.K2_GetActorLocation`) 0.0 500.0 true)
    (`PrimitiveComponent.SetCollisionEnabled` (`self.Sphere`) "NoCollision")
    (`PrimitiveComponent.SetCollisionEnabled` (`self.Capsule`) "NoCollision")))

(fn `UserConstructionScript`
  (set `self.weel` (`self.WheelBall`))
  (set `self.mesh` (`self.Capsule`))
  (set `self.bomb` (`self.WheelBall`)))